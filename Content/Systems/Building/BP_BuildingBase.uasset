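; Base Blueprint for modular building pieces, handling placement validation and socket visibility.
; CanBePlaced extends parent checks with foundation ground traces, forced overlap queries, ignore lists, same-location upgrade detection and snapping rules.
; PlaceOnSocket spawns a temporary brush to test overlaps, then swaps it for an instanced module via AddModule and consumes resources.
; Hardcoded literals disable the blocker-volume, spline-limit and inside-collision failures in CanBePlaced.
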(event `self.ReceiveBeginPlay`
  (if (not (`self.IsABrush`))
    (for _array_element (`self.K2_GetComponentsByClass` "/Script/Engine.ShapeComponent")
      (`PrimitiveComponent.SetCollisionEnabled` _array_element "NoCollision"))))

(event `BuildingTextInterface.OnBuildingTextUpdate`
  (params (Component :type "WidgetComponent Object Reference") (Enabled :type Boolean))
  (`SceneComponent.SetVisibility` Component Enabled false)
  (if Enabled
    (bind _asw_building_ghost_text (cast `/Game/UI/Building/W_BuildingGhostText` (`WidgetComponent.GetUserWidgetObject` Component)))
    (`/Game/UI/Building/W_BuildingGhostText.SetText` _asw_building_ghost_text (`self.TextRenderText`))
    (`WidgetComponent.RequestRedraw` Component)))

(event `self.ReceiveEndPlay`
  (params (EndPlayReason :type "EEndPlayReason Enum" :default "Destroyed")))

(event `self.ReceiveActorBeginOverlap`
  (params (OtherActor :type "Actor Object Reference")))

(event `self.ReceiveTick`
  (params (DeltaSeconds :type "Float (single-precision)")))

(event `ServerPlaceOnSocket`
  (params (`Target Socket Index` :type Integer) (`Building Class` :type "/Game/Systems/Building/BP_BuildingBase Class Reference") (`Building Socket Index` :type Integer))
  (`self.PlaceOnSocket` null (`KismetMathLibrary.MakeTransform` (0.0 0.0 0.0)))
  (`WorldPersistenceComponent.SaveActor` self))

(fn `CanBePlaced`
  (params (AttachTo :type "BuildableBase Object Reference") (InstanceIndex :type Integer))
  (returns (FailedMessage :type String) (ReturnValue :type "ECanBePlacedResult Enum"))
  (locals (FoundUpgradeable :type Boolean) (AboveGround :type Boolean) (OverlappingActorsHitResults :type "Array of HitResult Structure") (OverlappingActorsHitResultsCheckIgnore :type "Array of HitResult Structure") (LocalIgnoreBrush :type Boolean) (LocalFailedMessage :type String) (LocalFailedResult :type "ECanBePlacedResult Enum"))
  (bind _returnvalue (`self.K2_GetActorLocation`))
  (bind _instancedbuildingmesh (`self.InstancedBuildingMesh`))
  (bind _overlappingactorshitresults (`local.OverlappingActorsHitResults`))
  (bind _overlappingactorshitresultscheckignore (`local.OverlappingActorsHitResultsCheckIgnore`))
  (bind _instancedbuildingmesh_2 (`self.InstancedBuildingMesh`))
  (bind _returnvalue_location (`KismetMathLibrary.BreakTransform` (`SceneComponent.GetRelativeTransform` _instancedbuildingmesh)))
  (bind _returnvalue_2 (`SceneComponent.K2_GetComponentRotation` _instancedbuildingmesh))
  (bind (_failedmessage _returnvalue_3) (`parent.CanBePlaced` AttachTo InstanceIndex))
  (`|ExecutionSequence`
    (:`then_0`
      ;[1 0.6413 0.1882] Initialize Local Variables
      (`|ExecutionSequence`
        (:`then_0`
          (set `local.LocalFailedMessage` _failedmessage))
        (:`then_1`
          (set `local.LocalFailedResult` _returnvalue_3))
        (:`then_2`
          (set `local.LocalIgnoreBrush` false))))
    (:`then_1`
      (if (>= (`local.LocalFailedResult`) (enumliteral `ECanBePlacedResult` "Fail"))
        (return (`local.LocalFailedMessage`) (`local.LocalFailedResult`))
        (else
          ;[1 1 1] Check if above ground
          (if (`self.IsFoundation`)
            (bind _outhits (`KismetSystemLibrary.BoxTraceMultiForObjects` (+ (`KismetMathLibrary.GreaterGreater_VectorRotator` (+ (.location (`InstancedStaticMeshComponent.GetInstanceTransform` _instancedbuildingmesh 0 false)) _returnvalue_location) _returnvalue_2) _returnvalue) (- _returnvalue (0.0 0.0 10000.0)) (`self.UnderneathGround_Trace_HalfSize`) _returnvalue_2 (`|MakeArray` "ObjectTypeQuery1" :!type "EObjectTypeQuery Enum")))
            (bind _returnvalue_4 (`BuildableFunctionLibrary.HasStaticGroundInHitResults` _outhits))
            (set `local.AboveGround` _returnvalue_4))
          ;[1 1 1] Force generate overlap events
          (set `PrimitiveComponent.bForceGenerateOverlapEvents` true (`self.OverlapBuildingBoxChecker`))
          (set `PrimitiveComponent.bForceGenerateOverlapEvents` true (`self.InstancedBuildingMesh`))
          (set `PrimitiveComponent.bForceGenerateOverlapEvents` true (`self.OverlapPlaceablesBoxChecker`))
          (if (`self.UseSecondaryPlaceablesBoxChecker`)
            (set `PrimitiveComponent.bForceGenerateOverlapEvents` true (`self.SecondaryOverlapPlaceablesBoxChecker`)))
          (if (`self.UseSecondaryOverlapBuildingBoxChecker`)
            (set `PrimitiveComponent.bForceGenerateOverlapEvents` true (`self.SecondaryOverlapBuildingBoxChecker`)))
          (`FuncomGenericLibrary.UpdateOverlaps` self)
          ;[1 0.6413 0.1882] Bed Spawnpoint Overlap Check
          (bind _isblockingspawnpoints (`/Game/Systems/Building/BuildingFunctionLibrary.CheckOverlappingWithBedSpawnpoints` self (`local.LocalIgnoreBrush`)))
          (if _isblockingspawnpoints
            ;;[0.62 0 0] Fail: Overlapping with spawnpoints.
            (return (`KismetTextLibrary.Conv_TextToString` (`FuncomGenericLibrary.GetLocalizedBuildingBaseErrorText` "OverlappingSpawnpoints")) "Fail_Overlaps")
            (else
              (bind (_failedmessage_2 _isblocking) (`/Game/Characters/FuncomFunctionLibrary.IsOverlappingWithABuildingBlockerVolume` (`self.OverlapBuildingBoxChecker`)))
              (if (and _isblocking (not true))
                (return _failedmessage_2 "Fail")
                (else
                  (set `local.OverlappingActorsHitResults` (`FuncomGenericLibrary.GetOverlappingActorsAsHitResults` _instancedbuildingmesh_2 "/Script/Engine.Character"))
                  (`KismetArrayLibrary.Array_Append` _overlappingactorshitresults (`FuncomGenericLibrary.GetOverlappingActorsAsHitResults` _instancedbuildingmesh_2 "/Script/Foliage.InstancedFoliageActor"))
                  (`KismetArrayLibrary.Array_Append` _overlappingactorshitresults (`FuncomGenericLibrary.GetOverlappingActorsAsHitResults` _instancedbuildingmesh_2 "/Script/ConanSandbox.ResourceActorBase"))
                  (set `local.OverlappingActorsHitResultsCheckIgnore` (`FuncomGenericLibrary.GetOverlappingActorsAsHitResults` (`self.OverlapBuildingBoxChecker`) "/Script/ConanSandbox.BuildableBase"))
                  (if (`self.UseSecondaryOverlapBuildingBoxChecker`)
                    ;[1 1 1] Secondary Building Box Overlap
                    (`KismetArrayLibrary.Array_Append` (`local.OverlappingActorsHitResultsCheckIgnore`) (`FuncomGenericLibrary.GetOverlappingActorsAsHitResults` (`self.SecondaryOverlapBuildingBoxChecker`) "/Script/ConanSandbox.BuildableBase"))
                    (set `PrimitiveComponent.bForceGenerateOverlapEvents` false (`self.SecondaryOverlapBuildingBoxChecker`)))
                  (`KismetArrayLibrary.Array_Append` (`local.OverlappingActorsHitResultsCheckIgnore`) (`FuncomGenericLibrary.GetOverlappingActorsAsHitResults` (`self.OverlapPlaceablesBoxChecker`) "/Script/ConanSandbox.PlaceableBase"))
                  (`self.RemoveIgnoredStaticMeshHits` _overlappingactorshitresultscheckignore)
                  (`KismetArrayLibrary.Array_Append` (`local.OverlappingActorsHitResults`) _overlappingactorshitresultscheckignore)
                  (if (`self.UseSecondaryPlaceablesBoxChecker`)
                    (`KismetArrayLibrary.Array_Append` (`local.OverlappingActorsHitResults`) (`FuncomGenericLibrary.GetOverlappingActorsAsHitResults` (`self.SecondaryOverlapPlaceablesBoxChecker`) "/Script/ConanSandbox.PlaceableBase"))
                    (set `PrimitiveComponent.bForceGenerateOverlapEvents` false (`self.SecondaryOverlapPlaceablesBoxChecker`)))
                  (set `PrimitiveComponent.bForceGenerateOverlapEvents` false (`self.OverlapPlaceablesBoxChecker`))
                  (bind _foundupgrade (`self.PruneUpgradeHits` (`local.OverlappingActorsHitResults`)))
                  (set `local.FoundUpgradeable` _foundupgrade)
                  (if (or (`local.FoundUpgradeable`) (== (`KismetArrayLibrary.Array_Length` (`local.OverlappingActorsHitResults`)) 0))
                    (if (`self.MustSnapToExistingBuilding`)
                      (if (`self.IsSnappedToSocket`)
                        _
                        (else
                          (return (`KismetTextLibrary.Conv_TextToString` (`FuncomGenericLibrary.GetLocalizedBuildingBaseErrorText` "NotSnapped")) "Fail"))))
                    (if (`local.FoundUpgradeable`)
                      (if (< (`local.LocalFailedResult`) (enumliteral `ECanBePlacedResult` "Fail"))
                        (return "" "Success_Update")
                        (else
                          _)))
                    (bind _returnvalue_5 (`self.IsInAllowedSplineBuildLimit`))
                    (if (or _returnvalue_5 true)
                      (if false
                        (return (`KismetTextLibrary.Conv_TextToString` (`FuncomGenericLibrary.GetLocalizedBuildingBaseErrorText` "InsideCollision")) "Fail_InsideCollision")
                        (elif (or (`local.AboveGround`) (not (`self.IsFoundation`)))
                          (return (`local.LocalFailedMessage`) (`local.LocalFailedResult`))
                          (else
                            (return (`KismetTextLibrary.Conv_TextToString` (`FuncomGenericLibrary.GetLocalizedBuildingBaseErrorText` "BelowGround")) "Fail"))))
                      (else
                        (return (`KismetTextLibrary.Conv_TextToString` (`FuncomGenericLibrary.GetLocalizedBuildingBaseErrorText` "DisallowedSplineBuildLimit")) "Fail_DisallowedBuildLimit")))
                    (else
                      (set `self.LastCanBePlacedOverlapResults` (`local.OverlappingActorsHitResults`))
                      (return (`KismetTextLibrary.Conv_TextToString` (`FuncomGenericLibrary.GetLocalizedBuildingBaseErrorText` "Overlapping_Text")) "Fail_Overlaps"))))))))))))

(fn `HideAllSockets`
  (`SceneComponent.SetHiddenInGame` (`self.BuildSockets`) true true))

(fn `IsInAllowedSplineBuildLimit`
  (returns (ReturnValue :type Boolean))
  (`parent.IsInAllowedSplineBuildLimit`)
  (bind _isallowed (`/Game/Characters/FuncomFunctionLibrary.IsInAllowedBuildSplineLimit` self (`self.K2_GetActorLocation`) self))
  (return _isallowed))

(fn `PlaceOnSocket`
  (params (`Building Class` :type "BuildingBase Class Reference") (TargetTransform :type "Transform Structure") (OwnerSystem :type "BuildSystemComponent Object Reference"))
  (locals (LocalMeshTransform :type "Transform Structure") (AnnoyingWorkAround :type Boolean :default true))
  (bind _asconan_character (cast `ConanCharacter` (`ActorComponent.GetOwner` OwnerSystem) :!pure true))
  (bind _asbp_building_base (castclass `/Game/Systems/Building/BP_BuildingBase` `Building Class`)
    (:`then`
      (bind _returnvalue (`|SpawnActorFromClass` `Building Class` TargetTransform "AlwaysSpawn" "OverrideRootScale" null null 0 (`local.AnnoyingWorkAround`) true (`ConanCharacter.GetPrioritizedUID` _asconan_character)))
      (bind _asbp_building_base_2 (cast `/Game/Systems/Building/BP_BuildingBase` _returnvalue)
        (:`then`
          (`self.SetReplicates` _asbp_building_base_2 false)
          (set `BuildableBase.IsABrush` true _asbp_building_base_2)
          (bind _overlappingactors (`self.GetOverlappingActors` _asbp_building_base_2 "/Script/ConanSandbox.BuildingBase"))
          (bind _returnvalue_2 (`KismetArrayLibrary.Array_Length` _overlappingactors))
          (if (not (<= _returnvalue_2 0))
            (bind _asbp_building_base_3 (cast `/Game/Systems/Building/BP_BuildingBase` (`KismetArrayLibrary.Array_Get` _overlappingactors))
              (:`then`
                (if (and (`BuildingBase.IsABrush` _asbp_building_base_3) (<= _returnvalue_2 1))
                  _
                  (else
                    (`KismetSystemLibrary.PrintString` (`KismetTextLibrary.Conv_TextToString` (`|FormatText` "Can't place there, overlapping: {a}" (`KismetTextLibrary.Conv_IntToText` _returnvalue_2))) :!label _label)
                    (`self.K2_DestroyActor` _asbp_building_base_2)
                    (return))))
              (:`CastFailed`
                (goto _label))))
          (bind _canconsume (message `/Game/Systems/Building/BuildSystemInterface.CanConsumeResources` OwnerSystem))
          (if _canconsume
            (bind _instancedbuildingmesh (`BuildingBase.InstancedBuildingMesh` _asbp_building_base_2))
            (bind _returnvalue_3 (`KismetMathLibrary.ComposeRotators` (.rotation (`InstancedStaticMeshComponent.GetInstanceTransform` _instancedbuildingmesh 0 false)) (`KismetMathLibrary.ComposeRotators` (.rotation (`SceneComponent.GetRelativeTransform` _instancedbuildingmesh)) (.rotation TargetTransform))))
            (bind _output_get (set `local.LocalMeshTransform` (`KismetMathLibrary.MakeTransform` (+ (.location TargetTransform) (.location (`SceneComponent.GetRelativeTransform` _instancedbuildingmesh)) (`KismetMathLibrary.GreaterGreater_VectorRotator` (.location (`InstancedStaticMeshComponent.GetInstanceTransform` _instancedbuildingmesh 0 false)) _returnvalue_3)) _returnvalue_3 (* (.scale (`SceneComponent.GetRelativeTransform` _instancedbuildingmesh)) (.scale (`InstancedStaticMeshComponent.GetInstanceTransform` _instancedbuildingmesh 0 false))))))
            (message `/Game/Systems/Building/BuildSystemInterface.PlayPlacementSoundWithLocation` OwnerSystem self (.location TargetTransform))
            (`self.K2_DestroyActor` _asbp_building_base_2)
            (bind _returnvalue_4 (`self.AddModule` _asbp_building_base TargetTransform _output_get (`|MakeArray`) 0 (make `UpdateDecayContext` false true) (`ConanCharacter.GetPrioritizedUID` _asconan_character)))
            (if _returnvalue_4
              (message `/Game/Systems/Building/BuildSystemInterface.ConsumeResources` OwnerSystem)
              (else
                (bind _asconan_player_controller (cast `ConanPlayerController` (`Pawn.GetController` _asconan_character) :!label _label_2)
                  (:`then`
                    (`/Engine/EditorBlueprintResources/StandardMacros.IsValid` _asconan_player_controller
                      (:`Is Valid`
                        (`ConanPlayerController.ClientHUDShowNotification` _asconan_player_controller "Failed to place building" false))
                      (:`Is Not Valid`
                        _)))
                  (:`CastFailed`
                    _))))
            (else
              (`KismetSystemLibrary.PrintString` "Couldn't consume resources.")
              (`self.K2_DestroyActor` _asbp_building_base_2)
              (goto _label_2)))
          (`WorldPersistenceComponent.SaveActor` self)
          (return))
        (:`CastFailed`
          (return))))
    (:`CastFailed`
      (return))))

(fn `PruneUpgradeHits`
  (params (ListToPrune :type "Array of HitResult Structure (by ref)"))
  (returns (FoundUpgrade :type Boolean))
  (locals (PrunedList :type "Array of HitResult Structure") (localFoundUpgrade :type Boolean))
  (for _array_element ListToPrune
    (bind (_bblockinghit _binitialoverlap _time _location _impactpoint _normal _impactnormal _physmat _hitactor _hitcomponent _hitbonename _hititem) (`GameplayStatics.BreakHitResult` _array_element))
    (bind _asinstanced_building_component (cast `InstancedBuildingComponent` _hitcomponent)
      (:`then`
        (if (or (`KismetArrayLibrary.Array_Contains` (`self.CanUpgradeFrom`) (`StaticMeshComponent.StaticMesh` _asinstanced_building_component)) (`self.CanUpgradeFromTagContainer` (`BuildingBase.CanUpgradeFromTagList` (`DreamworldBlueprints.GetClassDefaultObject` (`InstancedBuildingComponent.m_SourceClass` _asinstanced_building_component)))))
          (if (== (.location (`InstancedStaticMeshComponent.GetInstanceTransform` _asinstanced_building_component _hititem true)) (.location (`InstancedStaticMeshComponent.GetInstanceTransform` (`self.InstancedBuildingMesh`) 0 true)) :`ErrorTolerance` 1.0)
            (set `local.localFoundUpgrade` true)
            (else
              (`KismetArrayLibrary.Array_Add` (`local.PrunedList`) _array_element :!label _label)))
          (else
            (goto _label))))
      (:`CastFailed`
        (`KismetArrayLibrary.Array_Add` (`local.PrunedList`) _array_element))))
  (`|VariableSetRef` ListToPrune (`local.PrunedList`))
  (return (`local.localFoundUpgrade`)))

(fn `RemoveIgnoredStaticMeshHits`
  (params (ListToPrune :type "Array of HitResult Structure (by ref)"))
  (locals (PrunedList :type "Array of HitResult Structure") (ShouldBeIgnored :type Boolean))
  (for _array_element ListToPrune
    (bind (_bblockinghit _binitialoverlap _time _location _impactpoint _normal _impactnormal _physmat _hitactor _hitcomponent) (`GameplayStatics.BreakHitResult` _array_element))
    (bind _asbuildable_base (cast `BuildableBase` _hitactor)
      (:`then`
        (if (not (`BuildableBase.IsABrush` _asbuildable_base))
          (`/Engine/EditorBlueprintResources/StandardMacros.IsValid` _hitcomponent :!label _label
            (:`Is Valid`
              (set `local.ShouldBeIgnored` false)
              (bind _asinstanced_building_component (cast `InstancedBuildingComponent` _hitcomponent)
                (:`then`
                  (for _array_element_2 (`self.IgnoreOverlappingTheseBuildableModules`)
                    (if (`KismetMathLibrary.ClassIsChildOf` (`InstancedBuildingComponent.m_SourceClass` _asinstanced_building_component) _array_element_2)
                      (set `local.ShouldBeIgnored` true)
                      (break)))
                  (if (not (`local.ShouldBeIgnored`))
                    (`KismetArrayLibrary.Array_Add` (`local.PrunedList`) _array_element)))
                (:`CastFailed`
                  (`KismetArrayLibrary.Array_Add` (`local.PrunedList`) _array_element))))
            (:`Is Not Valid`
              (`KismetArrayLibrary.Array_Add` (`local.PrunedList`) _array_element)))))
      (:`CastFailed`
        (goto _label))))
  (`|VariableSetRef` ListToPrune (`local.PrunedList`)))

(fn `ShowSockets`
  (params (SocketTypeToShow :type "/Game/Systems/Building/Enum_BuildingSocketTypes Enum"))
  (bind _returnvalue (`self.K2_GetComponentsByClass` (`GameplayStatics.GetPlayerPawn` 0) "/Script/ConanSandbox.BuildSystemComponent"))
  (if (> (`KismetArrayLibrary.Array_Length` _returnvalue) 0)
    (if (`BuildSystemComponent.ShowBuildingSockets` (`KismetArrayLibrary.Array_Get` _returnvalue))
      (`SceneComponent.SetHiddenInGame` (`self.BuildSockets`) false true))))

(fn `UserConstructionScript`)