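; Player component for placing thralls, pets and mounts from inventory items or moving existing ones.
; Tick moves a non-replicated preview brush along a camera trace, showing blocked reasons in the HUD.
; Server events validate collision and navigation, then teleport the thrall or spawn and configure an NPC, consume the item and fire journey events.
; CheckValidPlacement's exclusion-radius checks are disconnected and its build-spline result is unused.
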(event `self.ReceiveTick`
  (params (DeltaSeconds :type "Float (single-precision)"))
  (bind _returnvalue (`GUIModuleController.GetGUIModuleController`))
  (bind _brushactor (`self.BrushActor`))
  ;[1 1 1] EventTick
  (if (`self.IsPlacingThrall`)
    (`|ExecutionSequence`
      (:`then_0`
        (bind _asbase_player_char_interface (cast `/Game/Systems/Interfaces/BasePlayerCharInterface` (`self.GetOwner`)))
        (bind _value (`/Game/Systems/Interfaces/BasePlayerCharInterface.GetCameraActive` _asbase_player_char_interface))
        (bind _returnvalue_2 (`SceneComponent.K2_GetComponentLocation` _value))
        (bind _outhit (`KismetSystemLibrary.SphereTraceSingle` _returnvalue_2 (+ _returnvalue_2 (* (`SceneComponent.GetForwardVector` _value) (`self.PlaceableRange`))) 0.0 "TraceTypeQuery1" false (`|MakeArray` (`self.BrushActor`))))
        (bind _output_get (set `self.BrushTransform` (`KismetMathLibrary.MakeTransform` (+ (`.Location` (`GameplayStatics.BreakHitResult` _outhit)) (`KismetMathLibrary.MakeVector` 0.0 0.0 (`self.BrushGroundOffset`))) (`KismetMathLibrary.ComposeRotators` (`Actor.K2_GetActorRotation` (`self.GetOwner`)) (`self.Rotation`)) (1.0 1.0 1.0))))
        (`Actor.K2_SetActorTransform` _brushactor _output_get false false)
        (bind (_debugtext _displayfailtext _returnvalue_3) (`self.CanBePlaced` (`KismetArrayLibrary.Array_Get` (`Actor.K2_GetComponentsByClass` _brushactor "/Script/ConanSandbox.ThrallComponent"))))
        (if (`|EnumEquality` _returnvalue_3 "Success")
          (`GUIModuleController.ActivateModule` _returnvalue "CanBuildIndicator" false false)
          (else
            (bind _returnvalue_4 (`GUIModuleController.ActivateModule` _returnvalue "CanBuildIndicator" true false))
            (bind _asw_can_build_indicator (cast `/Game/UI/Building/W_CanBuildIndicator` _returnvalue_4))
            (`/Game/UI/Building/W_CanBuildIndicator.SetBlockedReason` _asw_can_build_indicator _displayfailtext))))
      (:`then_1`
        ;[1 0.06667 0] TEMPORARY SOLUTION. Because thrall will no longer exist on the client if you move too far away, you won't be able to place it. We should fix this. Also there is an issue with teleporting actors suspended by the AILOD system
        (switch `EThrallPlacementMode` (`self.ThrallPlacementMode`)
          (:`MoveExistingThrall`
            (`/Engine/EditorBlueprintResources/StandardMacros.IsValid` (`self.CurrentThrallComponent`)
              (:`Is Not Valid`
                (bind _asconan_player_controller (cast `ConanPlayerController` (`/Game/Characters/FuncomFunctionLibrary.GetControllerFromActor` (`self.GetOwner`))))
                (`ConanPlayerController.ClientHUDShowNotification` _asconan_player_controller "Too far away." false)
                (`self.StopPlacingThrall` null)))))))))

(event `Server Place Thrall`
  (params (WorldPosition :type "Transform Structure") (ThrallItemInventory :type "ItemInventory Object Reference") (ThrallItemIndex :type Integer))
  ;[1 1 1] ServerPlaceThrall
  (`self.PlaceThrallInternal` WorldPosition ThrallItemInventory ThrallItemIndex))

(event `ServerTeleportThrall`
  (params (Thrall :type "ThrallComponent Object Reference") (NewTransform :type "Transform Structure"))
  (bind _returnvalue (`self.GetOwner` Thrall))
  (bind _location (.location NewTransform))
  (set `self.ThrallPlacementMode` "MoveExistingThrall")
  (if (`/Game/Characters/FuncomFunctionLibrary.HasOwnership` _returnvalue (`self.GetOwner`))
    (bind (_valid _debugtext _displayfailtext) (`self.CheckValidPlacement` (.location NewTransform) true _returnvalue))
    (if _valid
      (bind _returnvalue_2 (`self.IsValidPlacementLocationOnNavigation` (.location NewTransform) Thrall))
      (`self.ServerRegisterPlayerAsNavigationInvoker` false)
      (if _returnvalue_2
        (`Actor.K2_SetActorLocationAndRotation` (`self.GetOwner` Thrall) _location (.rotation NewTransform) false false)
        (`self.Play Placement Sound` _location)
        (`ThrallComponent.OnThrallPlaced` Thrall)
        (bind (_debugtext_2 _displayfailtext_2 _returnvalue_3) (`self.CanBePlaced` Thrall))
        (if (not (`|EnumEquality` _returnvalue_3 "Success"))
          (bind _asconan_character (cast `ConanCharacter` (`self.GetOwner`)))
          (`ConanCharacter.ClientHUDShowFIFO` _asconan_character _displayfailtext_2))
        (else
          (bind _asconan_character_2 (cast `ConanCharacter` (`self.GetOwner`)))
          (`ConanCharacter.ClientHUDShowFIFO` _asconan_character_2 "Must be placed on walkable floor")))
      (else
        (bind _asconan_character_3 (cast `ConanCharacter` (`self.GetOwner`)))
        (`ConanCharacter.ClientHUDShowFIFO` _asconan_character_3 _displayfailtext)))))

(event `Play Placement Sound`
  (params (Location :type "Vector Structure"))
  (if (not (`KismetSystemLibrary.IsDedicatedServer`))
    (`DreamworldBlueprints.PlaySoundAtLocation` "/Game/Sound/SFX/Building/Placeables/sfx_placeable_pet_Cue.sfx_placeable_pet_Cue" Location)))

(fn `CanBePlaced`
  (params (ThrallComponent :type "ThrallComponent Object Reference"))
  (returns (DebugText :type String) (DisplayFailText :type Text) (ReturnValue :type "EThrallCanBePlacedResult Enum"))
  (bind _returnvalue (`self.GetOwner` ThrallComponent))
  (bind (_debugtext _displayfailtext _returnvalue_2) (`parent.CanBePlaced` ThrallComponent))
  (if (`|EnumInequality` _returnvalue_2 "Success")
    (return _debugtext _displayfailtext _returnvalue_2)
    (else
      (bind (_debugtext_2 _displayfailtext_2 _returnvalue_3) (`self.CheckTargetLocationForBuildings` _returnvalue (`Actor.K2_GetActorLocation` _returnvalue)))
      (return _debugtext_2 _displayfailtext_2 _returnvalue_3))))

(fn `CheckTargetLocation`)

(fn `CheckTargetLocationForBuildings`
  (params (PlacingActor :type "Actor Object Reference") (TargetLocation :type "Vector Structure") (IgnoreBuildingBlockerVolumes :type Boolean))
  (returns (DebugText :type String) (DisplayFailText :type Text) (ReturnValue :type "EThrallCanBePlacedResult Enum"))
  (bind (_debugtext _displayfailtext _returnvalue) (`parent.CheckTargetLocationForBuildings` PlacingActor TargetLocation IgnoreBuildingBlockerVolumes))
  (bind (_outactors _returnvalue_2) (`KismetSystemLibrary.BoxOverlapActors` (0.0 0.0 0.0) (64.0 64.0 32.0) (`|MakeArray` "ObjectTypeQuery10" :!type "EObjectTypeQuery Enum") "/Script/ConanSandbox.BuildableBase"))
  (if _returnvalue_2
    (return "" (`self.Error: Overlapping with a placed object`) "Fail_Overlaps")
    (elif (`|EnumInequality` _returnvalue "Success")
      (return _debugtext _displayfailtext _returnvalue)
      (else
        (bind (_valid _debugtext_2 _displayfailtext_2) (`self.CheckValidPlacement` TargetLocation (`KismetSystemLibrary.IsServer`) PlacingActor))
        (if _valid
          (if (not IgnoreBuildingBlockerVolumes)
            (`/Game/Characters/FuncomFunctionLibrary.GetCanBypassBuildingBlockerVolumes` self)
            (if (not true)
              (bind (_outactors_2 _returnvalue_3) (`KismetSystemLibrary.BoxOverlapActors` TargetLocation (64.0 64.0 32.0) (`|MakeArray` "ObjectTypeQuery4" :!type "EObjectTypeQuery Enum") "/Game/Systems/Building/BuildingBlockerVolume.BuildingBlockerVolume_C"))
              (if _returnvalue_3
                (bind _asbuilding_blocker_volume (cast `/Game/Systems/Building/BuildingBlockerVolume` (`KismetArrayLibrary.Array_Get` _outactors_2))
                  (:`then`
                    (for _array_element (`SpecialPropertiesVolume.Whitelist` _asbuilding_blocker_volume)
                      (if (`KismetMathLibrary.ClassIsChildOf` (`GameplayStatics.GetObjectClass` PlacingActor) (`|ConvertAsset` _array_element))
                        (return "" "" "Success")))
                    (return (`KismetTextLibrary.Conv_TextToString` "Invalid placement location") "Invalid placement location" "Fail_LandClaim"))
                  (:`CastFailed`
                    _)))))
          (return "" "" "Success")
          (else
            (return _debugtext_2 _displayfailtext_2 "Fail")))))))

(fn `CheckValidPlacement`
  (params (Location :type "Vector Structure") (IsServer :type Boolean) (PlacingActor :type "Actor Object Reference"))
  (returns (Valid :type Boolean) (DebugText :type String) (DisplayFailText :type Text))
  (locals (ThrallActors :type "Array of Actor Object Reference") (localLocation :type "Vector Structure") (TooCloseDebugString :type String :default "Failed due to existing thralls being within the exclusion zone") (TooCloseDisplayText :type Text :default "NSLOCTEXT(\"\", \"5FA8380D4D802A1258AF0696661C8D32\", \"Too close to another Thrall\")"))
  (bind (_asconan_character _bsuccess) (cast `ConanCharacter` PlacingActor :!pure true))
  (bind _output_get (set `local.localLocation` Location))
  (bind _isallowed (`/Game/Characters/FuncomFunctionLibrary.IsInAllowedBuildSplineLimit` self _output_get PlacingActor))
  (bind _canbypassbuildingblockervolumes (`/Game/Characters/FuncomFunctionLibrary.GetCanBypassBuildingBlockerVolumes` self))
  (if true
    (if _bsuccess
      (if (`KismetSystemLibrary.IsValid` (`ConanCharacter.GetRider` _asconan_character))
        (return false "Failed to place, mount currently being ridden" "Cannot move a mount with rider")
        (else
          _)))
    (bind _returnvalue (`FuncomGenericLibrary.IsPointCompletelyInsideCollision` (`local.localLocation`) (`|MakeArray` PlacingActor) false (0.0 0.0 5000.0)))
    (if (not _returnvalue)
      (if IsServer
        (return true "" "")
        (else
          ;[1 1 1] On the client let's just check every NPC we have, current location of the NPC. We don't have their home location here.
          (return true "" "")))
      (else
        (return false "Failed to place, thrall is inside collision" "Thrall is inside collision")))
    (else
      (return false "Failed to place, thrall is inside build spline limit" "Thralls are not allowed here"))))

(fn `GetPlacementThrallCharacterLayout`
  (returns (ReturnValue :type "CharacterLayout Structure"))
  (bind _currentthrallitem (`self.CurrentThrallItem`))
  (switch `EThrallPlacementMode` (`self.ThrallPlacementMode`)
    (:`None`
      _)
    (:`PlaceNewThrall`
      (`/Engine/EditorBlueprintResources/StandardMacros.IsValid` _currentthrallitem
        (:`Is Valid`
          (return (`ThrallItem.ThrallCharLayout` _currentthrallitem)))
        (:`Is Not Valid`
          _)))
    (:`MoveExistingThrall`
      (bind _character_layout (message `/Game/Characters/I_HasCharacterLayoutInterface.GetCharacterLayout` (`self.GetOwner` (`self.CurrentThrallComponent`))))
      (return _character_layout)))
  (bind _returnvalue (`parent.GetPlacementThrallCharacterLayout`))
  (return _returnvalue))

(fn `HideThrallPlaceable`
  (returns (ReturnValue :type Boolean))
  (`Actor.K2_DestroyActor` (`self.BrushActor`))
  (`self.SetIsBuildingThrall` false)
  (bind _returnvalue (`parent.HideThrallPlaceable`))
  (`GUIModuleController.ActivateModule` (`GUIModuleController.GetGUIModuleController`) "CanBuildIndicator" false false)
  (return _returnvalue))

(fn `OnPlacementAddJourneyEvent`
  (params (ThrallInfo :type "ThrallInfo Structure (by ref)"))
  (bind _returnvalue (`self.GetOwner`))
  (if (`KismetSystemLibrary.IsServer`)
    ;[1 1 1] Bandit chief Sennu
    (if (`DreamworldBlueprints.IsInTrialMode`)
      (if (`KismetStringLibrary.Contains` (`KismetTextLibrary.Conv_TextToString` (`.ThrallName` (break `ThrallInfo` ThrallInfo))) "Sennu")
        (`ExilesJourneyComponent.AddJourneyEvent` (`Actor.GetComponentByClass` _returnvalue "/Game/Systems/Progression/BP_AC_ExilesJourney.BP_AC_ExilesJourney_C") "EnslaveBanditChief" (`Actor.K2_GetActorLocation` _returnvalue))))))

(fn `PlaceThrall`
  (returns (ReturnValue :type Boolean))
  (bind _currentthrallcomponent (`self.CurrentThrallComponent`))
  (bind _returnvalue (`Actor.GetComponentsByTag` (`self.GetOwner`) "/Script/ConanSandbox.ItemInventory" "ShortcutBar"))
  (bind _item (`KismetArrayLibrary.Array_Get` _returnvalue))
  (bind (_debugtext _displayfailtext _returnvalue_2) (`self.CanBePlaced` (`KismetArrayLibrary.Array_Get` (`Actor.K2_GetComponentsByClass` (`self.BrushActor`) "/Script/ConanSandbox.ThrallComponent"))))
  (if (`|EnumEquality` _returnvalue_2 "Success")
    (`Actor.K2_DestroyActor` (`self.BrushActor`))
    (switch `EThrallPlacementMode` (`self.ThrallPlacementMode`)
      (:`None`
        _)
      (:`PlaceNewThrall`
        (if (> (`KismetArrayLibrary.Array_Length` _returnvalue) 0)
          (`self.Server Place Thrall` (`self.BrushTransform`) _item (`ItemInventory.GetItemIndex` _item (`self.CurrentThrallItem`)))
          (else
            (`LoggerLibrary.DWLogString` "PlaceThrall: Can't find ShorcutBar" "Thrall" "INFOL_DATAERROR")))
        (set `self.IsPlacingThrall` false :!label _label)
        (set `self.BrushActor` null)
        (set `self.ThrallPlacementMode` "None")
        (bind _returnvalue_3 (`parent.PlaceThrall`))
        (return _returnvalue_3))
      (:`MoveExistingThrall`
        (`/Engine/EditorBlueprintResources/StandardMacros.IsValid` _currentthrallcomponent
          (:`Is Valid`
            (`self.ServerTeleportThrall` _currentthrallcomponent (`self.BrushTransform`))
            (`self.HideThrallPlaceable`)
            (goto _label))
          (:`Is Not Valid`
            (return false))))))
  (return false))

(fn `PlaceThrallImplementation`
  (params (WorldPosition :type "Transform Structure") (ThrallItemInventory :type "ItemInventory Object Reference") (ThrallItemIndex :type Integer))
  (locals (`Local World Position` :type "Transform Structure") (`Local Thrall Item Inventory` :type "ItemInventory Object Reference") (`Local Thrall Item Index` :type Integer))
  (bind _sourcethrallitem (`self.SourceThrallItem`))
  (bind _sourcethrallitem_2 (`self.SourceThrallItem`))
  (bind _spawnedactor (`self.SpawnedActor`))
  (bind _local_thrall_item_inventory (`local.Local Thrall Item Inventory`))
  (bind _spawnedactor_2 (`self.SpawnedActor`))
  (bind _location (.location (`local.Local World Position`)))
  (bind _returnvalue (`Actor.GetComponentByClass` (`self.SpawnedActor`) "/Script/UE4Dreamworld.ActorPersistenceComponent"))
  (bind _returnvalue_2 (`ItemInventory.GetItem` _local_thrall_item_inventory (`local.Local Thrall Item Index`)))
  (bind _thrallinfo (`ThrallItem.ThrallInfo` _sourcethrallitem_2))
  (bind _object (`|ConvertAsset` (`ThrallItem.GetAIControllerClass` _sourcethrallitem)))
  (`|ExecutionSequence`
    (:`then_0`
      (set `local.Local World Position` WorldPosition)
      (set `local.Local Thrall Item Inventory` ThrallItemInventory)
      (set `local.Local Thrall Item Index` ThrallItemIndex)
      (set `self.ThrallPlacementMode` "PlaceNewThrall"))
    (:`then_1`
      (`/Engine/EditorBlueprintResources/StandardMacros.IsValid` _local_thrall_item_inventory
        (:`Is Valid`
          (`/Engine/EditorBlueprintResources/StandardMacros.IsValid` _returnvalue_2
            (:`Is Valid`
              (bind _asthrall_item (cast `ThrallItem` _returnvalue_2)
                (:`then`
                  (set `self.SourceThrallItem` _asthrall_item)
                  (bind _valid (`self.CheckValidPlacement` _location true))
                  (if _valid
                    (bind _returnvalue_3 (`self.IsValidPlacementLocationOnNavigation` _location))
                    (`self.ServerRegisterPlayerAsNavigationInvoker` false)
                    (if _returnvalue_3
                      (`self.UpdateExilesJourney`)
                      (else
                        (bind _asconan_character (cast `ConanCharacter` (`self.GetOwner`))
                          (:`then`
                            (`ConanCharacter.ClientHUDShowFIFO` _asconan_character "Must be placed on walkable floor"))
                          (:`CastFailed`
                            _))
                        (return)))
                    (else
                      (bind _asconan_character_2 (cast `ConanCharacter` (`self.GetOwner`)))
                      (`ConanCharacter.ClientHUDShowFIFO` _asconan_character_2 "There's a thrall placed too close by"))))
                (:`CastFailed`
                  (`LoggerLibrary.DWLogString` "ServerPlaceThrall: Source item is not a thrall item" "Thrall" "INFOL_CODEWARNING")
                  (return))))
            (:`Is Not Valid`
              (`LoggerLibrary.DWLogString` "ServerPlaceThrall: Could not find chosen thrall item" "Thrall" "INFOL_CODEWARNING")
              (return))))
        (:`Is Not Valid`
          (`LoggerLibrary.DWLogString` "ServerPlaceThrall: Trying to spawn thrall from invalid inventory" "Thrall" "INFOL_CODEWARNING")
          (return))))
    (:`then_2`
      ;[1 1 1] Spawning an NPC
      (bind _returnvalue_4 (`self.SpawnThrall` _sourcethrallitem (select `bool` (`KismetSystemLibrary.IsValidClass` _object) :`false` "/Game/Systems/AI/NewAI/HumanAIController.HumanAIController_C" :`true` _object) (`local.Local World Position`)))
      (`/Engine/EditorBlueprintResources/StandardMacros.IsValid` _returnvalue_4
        (:`Is Valid`
          (set `self.SpawnedActor` _returnvalue_4)
          (bind _asconan_basic_aicontroller (cast `ConanBasicAIController` (`Pawn.GetController` _returnvalue_4))
            (:`then`
              (`ConanBasicAIController.UpdateBBKeysFromPawn` _asconan_basic_aicontroller)
              (`ThrallItem.SetupThrallFromItem` (`self.SourceThrallItem`) _returnvalue_4)
              (bind _returnvalue_5 (`ThrallItem.GetThrallTableRow` (`self.SourceThrallItem`)))
              (bind _asbase_npc (cast `/Game/Characters/BaseNPC` (`self.SpawnedActor`)))
              (bind _asbp_npcbehavior_parameters (castclass `/Game/Systems/AI/BP_NPCBehaviorParameters` (`|ConvertAsset` (`.NPCBehaviorParameters` (break `ThrallTableRow` _returnvalue_5)))))
              (bind _returnvalue_6 (`|GenericCreateObject` _asbp_npcbehavior_parameters (`self.SpawnedActor`)))
              (`/Game/Systems/AI/BP_AISpawningLibrary.ConfigureSpawnedNPC` "NewEnumerator3" true _asbase_npc 0 0 0 0.0 (`Actor.K2_GetActorLocation` _asbase_npc) null null _returnvalue_6 true "" (`.SpawnTableID` (break `ThrallInfo` (`ThrallItem.ThrallInfo` (`self.SourceThrallItem`)))))
              (`self.Play Placement Sound` (.location (`local.Local World Position`))))
            (:`CastFailed`
              (`LoggerLibrary.DWLogString` "ServerPlaceThrall: Tried to spawn an NPC that has no valid AIController" "Thrall" "INFOL_DATAERROR")
              (return))))
        (:`Is Not Valid`
          (`LoggerLibrary.DWLogString` "ServerPlaceThrall: SpawnThrall failed" "Thrall" "INFOL_DATAERROR")
          (return))))
    (:`then_3`
      (`self.RetriveUpdatedThrallPopulation`)
      (bind _returnvalue_7 (`UniqueID.GenerateUniqueID`))
      (`DreamworldBlueprints.SetUniqueID` (`self.SpawnedActor`) _returnvalue_7)
      (bind _returnvalue_8 (`self.FindOrSetupThrallComponent` _spawnedactor_2 (`ThrallItem.ThrallInfo` (`self.SourceThrallItem`))))
      (bind (_debugtext _displayfailtext _returnvalue_9) (`self.CanBePlaced` _returnvalue_8))
      (if (`|EnumEquality` _returnvalue_9 "Success")
        (bind _returnvalue_10 (`ThrallItem.GetThrallTableRow` _sourcethrallitem_2))
        (cast `/Game/Characters/BaseNPC` (`self.SpawnedActor`))
        (bind _asbp_thrall_component (cast `/Game/Systems/Thrall/BP_ThrallComponent` _returnvalue_8))
        (bind _asi_has_character_layout_interface (cast `/Game/Characters/I_HasCharacterLayoutInterface` _spawnedactor_2)
          (:`then`
            (`/Game/Characters/I_HasCharacterLayoutInterface.SetCharacterLayout` _asi_has_character_layout_interface (`ThrallItem.ThrallCharLayout` _sourcethrallitem_2) false))
          (:`CastFailed`
            _))
        (set `ThrallComponent.ThrallInfo` _thrallinfo _asbp_thrall_component)
        (bind _asconan_character_3 (cast `ConanCharacter` (`self.GetOwner`)))
        (`ThrallComponent.SetOwnerUniqueID` _asbp_thrall_component (`ConanCharacter.GetPrioritizedUID` _asconan_character_3))
        (bind _returnvalue_11 (`self.ConsumeThrallResource` (`self.SourceThrallItem`)))
        (if _returnvalue_11
          (`WorldPersistenceComponent.SaveActor` _spawnedactor)
          (`ThrallComponent.OnThrallPlaced` _returnvalue_8)
          (`self.OnPlacementAddJourneyEvent` _thrallinfo)
          (bind _asbase_npc_2 (cast `/Game/Characters/BaseNPC` (`self.SpawnedActor`)))
          (`/Game/Characters/BaseNPC.BeginPlay_SpawnProgressionAndAttributeComponents` _asbase_npc_2)
          (`/Engine/EditorBlueprintResources/StandardMacros.IsValid` _returnvalue
            (:`Is Valid`
              (`PersistenceComponent.SetDirty` _returnvalue true 5.0)))
          (else
            (`Actor.K2_DestroyActor` _spawnedactor)))
        (else
          (bind _asconan_character_4 (cast `ConanCharacter` (`self.GetOwner`))
            (:`then`
              (`ConanCharacter.ClientHUDShowFIFO` _asconan_character_4 _displayfailtext))
            (:`CastFailed`
              _))
          (`Actor.K2_DestroyActor` _spawnedactor_2))))
    (:`then_4`
      (return))))

(fn `RotateThrall`
  (params (Rotation :type "Float (double-precision)"))
  (set `self.Rotation` (`KismetMathLibrary.MakeRotator` (.roll (`self.Rotation`)) (.pitch (`self.Rotation`)) (+ (* Rotation 5.0) (.yaw (`self.Rotation`))))))

(fn `SetIsBuildingThrall`
  (params (isBuildingThrall :type Boolean))
  (bind _asconan_character (cast `ConanCharacter` (`self.GetOwner`)))
  (`/Engine/EditorBlueprintResources/StandardMacros.IsValid` _asconan_character
    (:`Is Valid`
      (`ConanCharacter.SetCharacterIsBuildingThrall` _asconan_character isBuildingThrall))))

(fn `ShowThrallPlaceable`
  (params (thrallInfo :type "ThrallInfo Structure (by ref)"))
  (returns (ReturnValue :type "Actor Object Reference"))
  (bind _brushactor (`self.BrushActor`))
  (bind _item (`KismetArrayLibrary.Array_Get` (`Actor.GetComponentsByTag` (`self.BrushActor`) "/Script/Engine.SkeletalMeshComponent" "MainMesh")))
  (bind _returnvalue (`parent.ShowThrallPlaceable` thrallInfo))
  (`GameplayStatics.SpawnSound2D` "/Game/Sound/SFX/Gui/gui_slot_get.gui_slot_get" 0.1)
  ;[1 1 1] If we already had a brush actor, destroy it when making a new one.
  (`/Engine/EditorBlueprintResources/StandardMacros.IsValid` _brushactor
    (:`Is Valid`
      (`Actor.K2_DestroyActor` _brushactor))
    (:`Is Not Valid`
      _))
  (bind _output_get (set `self.BrushActor` _returnvalue))
  (`Actor.SetReplicates` _output_get false)
  (`DreamworldBlueprints.SetUniqueID` (`self.BrushActor`) (`UniqueID.MakeNullUID`))
  (bind _returnvalue_2 (`self.GetPlacementThrallCharacterLayout`))
  (bind _asi_has_character_layout_interface (cast `/Game/Characters/I_HasCharacterLayoutInterface` (`self.BrushActor`))
    (:`then`
      (`/Game/Characters/I_HasCharacterLayoutInterface.SetCharacterLayout` _asi_has_character_layout_interface _returnvalue_2 false))
    (:`CastFailed`
      _))
  (bind _ascapsule_collision (cast `CapsuleComponent` (`Actor.K2_GetRootComponent` (`self.BrushActor`)))
    (:`then`
      (set `self.BrushGroundOffset` (`CapsuleComponent.GetScaledCapsuleHalfHeight` _ascapsule_collision)))
    (:`CastFailed`
      (set `self.BrushGroundOffset` 0.0)))
  (bind _asbase_bpchar_interface (cast `/Game/Systems/Interfaces/BaseBPCharInterface` (`self.BrushActor`))
    (:`then`
      (bind _isnpc (`/Game/Systems/Interfaces/BaseBPCharInterface.CheckIsNPC` _asbase_bpchar_interface))
      (if _isnpc
        (`Actor.SetActorEnableCollision` (`self.BrushActor`) false)
        (else
          (`PrimitiveComponent.SetCollisionEnabled` _item "NoCollision" :!label _label)
          (`SkeletalMeshComponent.PlayAnimation` _item "/Game/Characters/humans/animations/movement/male/normal/A_normal_idle_3rd_M.A_normal_idle_3rd_M" true))))
    (:`CastFailed`
      (goto _label)))
  (`self.SetIsBuildingThrall` true)
  (return (`self.BrushActor`)))

(fn `UpdateExilesJourney`
  (locals (LocalIsPet :type Text :default "INVTEXT(\"Pet\")") (LocalIsMount :type Text :default "INVTEXT(\"Mount\")"))
  (bind _sourcethrallitem (`self.SourceThrallItem`))
  (bind _returnvalue (`KismetTextLibrary.EqualEqual_TextText` (`GameItem.FirstModifier` _sourcethrallitem) (`local.LocalIsPet`)))
  (if (and (>= (`GameItem.GetIntStat` _sourcethrallitem "ThrallTier") 4) (not _returnvalue))
    (bind _asbase_player_char_interface (cast `/Game/Systems/Interfaces/BasePlayerCharInterface` (`self.GetOwner`))
      (:`then`
        (`/Game/Systems/Interfaces/BasePlayerCharInterface.AddJourneyEventInterfaceCall` _asbase_player_char_interface "RecruitAUniqueThrall")
        (`/Game/Systems/Interfaces/BasePlayerCharInterface.AddJourneyEventInterfaceCall` _asbase_player_char_interface "Siptah_RecruitAUniqueThrall"))
      (:`CastFailed`
        _))
    (elif _returnvalue
      (bind _asbase_player_char_interface_2 (cast `/Game/Systems/Interfaces/BasePlayerCharInterface` (`self.GetOwner`))
        (:`then`
          (`/Game/Systems/Interfaces/BasePlayerCharInterface.AddJourneyEventInterfaceCall` _asbase_player_char_interface_2 "Siptah_GetPet")
          (if (`KismetTextLibrary.EqualEqual_TextText` (`GameItem.SecondModifier` _sourcethrallitem) (`local.LocalIsMount`))
            (bind _asbase_player_char_interface_3 (cast `/Game/Systems/Interfaces/BasePlayerCharInterface` (`self.GetOwner`))
              (:`then`
                (`/Game/Systems/Interfaces/BasePlayerCharInterface.AddJourneyEventInterfaceCall` _asbase_player_char_interface_3 "Siptah_GetMount"))
              (:`CastFailed`
                _))))
        (:`CastFailed`
          _))))
  (return))